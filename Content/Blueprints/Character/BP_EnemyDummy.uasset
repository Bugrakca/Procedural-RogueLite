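; BP_EnemyDummy is an enemy dummy that reacts to damage, then dissolves and is destroyed when its health runs out.
; Attribute component health changes print current health; losses also stamp a TimeToHit material parameter, start a hit montage and run the death check.
; At zero health it disables mesh collision, waits briefly, then a timeline drives DissolveAmount on a dynamic material before destroying the actor.
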(event OnHealthChanged(BAttributeComp)
  (params (InstigatorActor :type Actor%20Object%20Reference) (OwningComp :type B%20Attribute%20Component%20Object%20Reference) (NewHealth :type Float%20%28single-precision%29) (Delta :type Float%20%28single-precision%29))
  (Development|PrintString (Utilities|String|ToString(Float) (Variables|/Script/ProceduralRoguelike.BAttributeComponent|GetHealth (Variables|Default|GetBAttributeComp))))
  (if (< Delta 0.0)
    (Rendering|Material|SetScalarParameterValueonMaterials (Variables|Default|GetSkeletalMesh) "TimeToHit" (Utilities|Time|GetTimeSeconds))
    (Animation|Montage|PlayMontage (Variables|Default|GetSkeletalMesh) "/Game/Blueprints/Character/Animations/AL_Standard_Anim_Rig_Hit_Chest_Montage.AL_Standard_Anim_Rig_Hit_Chest_Montage"
      (:then
        (CallFunction|Death)))))

(event Custom|Death
  (if (<= (Variables|/Script/ProceduralRoguelike.BAttributeComponent|GetHealth (Variables|Default|GetBAttributeComp)) 0.0)
    (Variables|Default|SetIsDead? true)
    (Collision|SetCollisionEnabled (Variables|Default|GetSkeletalMesh) "NoCollision")
    (Utilities|FlowControl|Delay 2.0)
    (CallFunction|SKMDissolve)))

(event Custom|SKMDissolve
  (bind _returnvalue (Rendering|Material|CreateDynamicMaterialInstance (Variables|Default|GetSkeletalMesh) 0 "/Game/Blueprints/Character/UEFN_Mannequin/SKM_UEFN_Mannequin/Materials/M_UEFN_Mannequin_Enemy_Inst.M_UEFN_Mannequin_Enemy_Inst" "None" :!class /Script/Engine.PrimitiveComponent))
  (Rendering|Material|SetMaterial (Variables|Default|GetSkeletalMesh) 0 _returnvalue)
  (bind _dissolvetrack (Timeline|Timeline_0 PlayFromStart)
    (:Update
      (Rendering|Material|SetScalarParameterValue _returnvalue "DissolveAmount" _dissolvetrack :!class /Script/Engine.MaterialInstanceDynamic))
    (:Finished
      (Actor|DestroyActor))))

(fn ConstructionScript)