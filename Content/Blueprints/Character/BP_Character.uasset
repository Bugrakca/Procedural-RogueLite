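; Player character Blueprint that runs a three-hit melee combo and adds a health widget to the viewport on begin play.
; A left mouse debug key starts the attack montages in sequence, or buffers input while an attack is running.
; CumboAttackSave plays the next montage if input was buffered, and ResetCombo clears the combo state.
; Health changes from the attributes component are printed to screen.
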(event OnHealthChanged(AttributesComp)
  (params (InstigatorActor :type Actor%20Object%20Reference) (OwningComp :type B%20Attribute%20Component%20Object%20Reference) (NewHealth :type Float%20%28single-precision%29) (Delta :type Float%20%28single-precision%29))
  (Development|PrintString (Utilities|String|ToString(Float) (Variables|/Script/ProceduralRoguelike.BAttributeComponent|GetHealth (Variables|Default|GetAttributesComp)))))

(event Custom|Cumbo%20Attack%20Save
  (bind _weaponspeed (Variables|Default|GetWeaponSpeed))
  (if (Variables|Default|GetbSaveAttack)
    (Variables|Default|SetbSaveAttack false)
    (switch int (Variables|Default|GetComboCounter)
      (:0
        (Variables|Default|SetComboCounter 1)
        (bind _output_get (Variables|Default|SetCurrentMontage "/Game/Blueprints/Character/Animations/Attack_PrimaryA_Montage.Attack_PrimaryA_Montage"))
        (Animation|Montage|PlayMontage (Variables|Character|GetMesh) _output_get _weaponspeed))
      (:1
        (Variables|Default|SetComboCounter 2)
        (bind _output_get_2 (Variables|Default|SetCurrentMontage "/Game/Blueprints/Character/Animations/Attack_PrimaryB_Montage.Attack_PrimaryB_Montage"))
        (Animation|Montage|PlayMontage (Variables|Character|GetMesh) _output_get_2 _weaponspeed))
      (:2
        (Variables|Default|SetComboCounter 0)
        (bind _output_get_3 (Variables|Default|SetCurrentMontage "/Game/Blueprints/Character/Animations/Attack_PrimaryC_Montage.Attack_PrimaryC_Montage"))
        (Animation|Montage|PlayMontage (Variables|Character|GetMesh) _output_get_3 _weaponspeed)))))

(event Custom|Reset%20Combo
  (Variables|Default|SetComboCounter 0)
  (Variables|Default|SetbSaveAttack false)
  (Variables|Default|SetbIsAttacking? false))

(event EventBeginPlay
  (bind _returnvalue (UserInterface|CreateWidget "/Game/UI/PlayerHealth_Widget.PlayerHealth_Widget_C"))
  (UserInterface|Viewport|AddtoViewport _returnvalue 0))

(event Collision|EventActorBeginOverlap
  (params (OtherActor :type Actor%20Object%20Reference)))

(event Input|MouseEvents|DebugKeyLeftMouseButton
  (params (Key :type Key%20Structure :default "None") (ActionValue :type Input%20Action%20Value%20Structure))
  (:Pressed
    (Variables|Default|SetWeaponSpeed 1.2)
    (if (Variables|Default|GetbIsAttacking?)
      (Variables|Default|SetbSaveAttack true)
      (else
        (Variables|Default|SetbIsAttacking? true)
        (switch int (Variables|Default|GetComboCounter)
          (:0
            (Variables|Default|SetComboCounter 1)
            (bind _output_get (Variables|Default|SetCurrentMontage "/Game/Blueprints/Character/Animations/Attack_PrimaryA_Montage.Attack_PrimaryA_Montage"))
            (Animation|Montage|PlayMontage (Variables|Character|GetMesh) _output_get (Variables|Default|GetWeaponSpeed)))
          (:1
            (Variables|Default|SetComboCounter 2)
            (bind _output_get_2 (Variables|Default|SetCurrentMontage "/Game/Blueprints/Character/Animations/Attack_PrimaryB_Montage.Attack_PrimaryB_Montage"))
            (Animation|Montage|PlayMontage (Variables|Character|GetMesh) _output_get_2 (Variables|Default|GetWeaponSpeed)))
          (:2
            (Variables|Default|SetComboCounter 0)
            (bind _output_get_3 (Variables|Default|SetCurrentMontage "/Game/Blueprints/Character/Animations/Attack_PrimaryC_Montage.Attack_PrimaryC_Montage"))
            (Animation|Montage|PlayMontage (Variables|Character|GetMesh) _output_get_3 (Variables|Default|GetWeaponSpeed))))))))

(fn ConstructionScript)