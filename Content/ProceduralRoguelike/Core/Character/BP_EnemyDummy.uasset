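; BP_EnemyDummy is a practice-style enemy that repeatedly swings a sword, reacts to damage and dissolves on death.
; On BeginPlay it spawns a BP_Sword, attaches it to the right-hand socket and starts a looping timer for attack montages.
; Health loss from BAttributeComp plays a hit montage, stamps a material hit-time parameter and checks for death.
; Death disables mesh collision, then a timeline drives a dynamic material dissolve before destroying enemy and weapon.
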(event OnHealthChanged(BAttributeComp)
  (params (InstigatorActor :type Actor%20Object%20Reference) (OwningComp :type B%20Attribute%20Component%20Object%20Reference) (NewHealth :type Float%20%28single-precision%29) (Delta :type Float%20%28single-precision%29))
  (Development|PrintString (Utilities|String|ToString(Float) (Variables|/Script/ProceduralRoguelike.BAttributeComponent|GetHealth (Variables|Default|GetBAttributeComp))) true true "(R=1.000000,G=0.027585,B=0.000000,A=1.000000)")
  (if (< Delta 0.0)
    (Animation|Montage|PlayMontage (Variables|Default|GetSkeletalMesh) "/Game/ProceduralRoguelike/Characters/Animations/AL_Standard_Anim_Rig_Hit_Chest_Montage.AL_Standard_Anim_Rig_Hit_Chest_Montage"
      (:then
        (Rendering|Material|SetScalarParameterValueonMaterials (Variables|Default|GetSkeletalMesh) "TimeToHit" (Utilities|Time|GetTimeSeconds))
        (CallFunction|Death)))))

(event Custom|Death
  (if (<= (Variables|/Script/ProceduralRoguelike.BAttributeComponent|GetHealth (Variables|Default|GetBAttributeComp)) 0.0)
    (Variables|Default|SetIsDead? true)
    (Collision|SetCollisionEnabled (Variables|Default|GetSkeletalMesh) "NoCollision")
    (Utilities|FlowControl|Delay 2.0)
    (CallFunction|SKMDissolve)))

(event Custom|SKMDissolve
  (bind _returnvalue (Rendering|Material|CreateDynamicMaterialInstance (Variables|Default|GetSkeletalMesh) 0 "/Game/ProceduralRoguelike/Characters/UEFN_Mannequin/SKM_UEFN_Mannequin/Materials/M_UEFN_Mannequin_Enemy_Inst.M_UEFN_Mannequin_Enemy_Inst" "None" :!class /Script/Engine.PrimitiveComponent))
  (Rendering|Material|SetMaterial (Variables|Default|GetSkeletalMesh) 0 _returnvalue)
  (bind _dissolvetrack (Timeline|Timeline_0 PlayFromStart)
    (:Update
      (Rendering|Material|SetScalarParameterValue _returnvalue "DissolveAmount" _dissolvetrack :!class /Script/Engine.MaterialInstanceDynamic))
    (:Finished
      (Actor|DestroyActor)
      (Actor|DestroyActor (Variables|Default|GetCurrentWeapon)))))

(event Custom|WeaponSwing
  (if (not (Variables|Default|GetIsDead?))
    (Animation|Montage|PlayMontage (Variables|Default|GetSkeletalMesh) "/Game/ProceduralRoguelike/Characters/Animations/Attack_PrimaryA_Montage.Attack_PrimaryA_Montage")))

(event EventBeginPlay
  (bind _returnvalue (Game|SpawnActorfromClass "/Game/ProceduralRoguelike/Core/Weapons/BP_Sword.BP_Sword_C" (Transformation|GetSocketTransform (Variables|Default|GetSkeletalMesh) "WeaponSocketR" "RTS_World") "AlwaysSpawn" "MultiplyWithRoot" 0 0))
  (bind _output_get (Variables|Default|SetCurrentWeapon _returnvalue))
  (Actor|SetOwner _output_get self)
  (Transformation|AttachComponentToComponent _output_get (Variables|Default|GetSkeletalMesh) "WeaponSocketR" "SnapToTarget" "SnapToTarget" "SnapToTarget" true)
  (Utilities|Time|SetTimerbyEvent (delegate Custom|WeaponSwing) 2.0 true))

(fn ConstructionScript)

(fn GetCurrentWeapon
  (bind _currentweapon (Variables|Default|GetCurrentWeapon))
  (Utilities|IsValid _currentweapon
    (:Is%20Valid
      (return _currentweapon))
    (:Is%20Not%20Valid
      (return 0))))